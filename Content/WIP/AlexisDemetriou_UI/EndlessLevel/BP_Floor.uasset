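; BP_Floor is a floor segment for an endless level, extending the track and speeding up the player as it is crossed.
; Construction builds two arrow-based spawn points, shuffles them and attaches a random number of child-actor obstacles, each from one of three random branches.
; A Box overlap calls ExtendFloor on the endless game mode and slightly raises the cube pawn's speed within a clamped range.
; GetAttachPoint exposes the Arrow's world transform.
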(event `self.Box.OnComponentBeginOverlap`
  (params (OverlappedComponent :type "PrimitiveComponent Object Reference") (OtherActor :type "Actor Object Reference") (OtherComp :type "PrimitiveComponent Object Reference") (OtherBodyIndex :type Integer) (bFromSweep :type Boolean) (SweepResult :type "HitResult Structure (by ref)"))
  (bind _asbp_endless_game_mode_base (cast `/Game/WIP/AlexisDemetriou_UI/EndlessLevel/BP_EndlessGameModeBase` (`GameplayStatics.GetGameMode`)))
  (`/Game/WIP/AlexisDemetriou_UI/EndlessLevel/BP_EndlessGameModeBase.Extend Floor` _asbp_endless_game_mode_base)
  (bind _asbp_endless_cube_pawn (cast `/Game/Blueprints/BP_EndlessCubePawn` (`GameplayStatics.GetPlayerPawn` 0)))
  (set `EndlessCubePawn.CurrentSpeed` (`KismetMathLibrary.FClamp` (* (`EndlessCubePawn.CurrentSpeed` _asbp_endless_cube_pawn) 1.01) 600.0 1000.0) _asbp_endless_cube_pawn))

(fn `Get AttachPoint`
  (returns (ReturnValue :type "Transform Structure"))
  (return (`SceneComponent.K2_GetComponentToWorld` (`self.Arrow`))))

(fn `Setup Spawn Points`
  (bind _returnvalue (`AddComponent|NODE_AddArrowComponent-2` :`RelativeTransform` (`KismetMathLibrary.MakeTransform` (`KismetMathLibrary.MakeVector` 0.0))))
  (`KismetArrayLibrary.Array_Add` (`self.Spawn Points`) (`SceneComponent.K2_GetComponentToWorld` _returnvalue))
  (bind _returnvalue_2 (`AddComponent|NODE_AddArrowComponent-4` :`RelativeTransform` (`KismetMathLibrary.MakeTransform` (`KismetMathLibrary.MakeVector` 0.0 100.0))))
  (`KismetArrayLibrary.Array_Add` (`self.Spawn Points`) (`SceneComponent.K2_GetComponentToWorld` _returnvalue_2)))

(fn `Spawn Obstacles`
  (locals (`Random Spawn Points` :type "Array of Transform Structure"))
  (bind _output_get (set `local.Random Spawn Points` (`self.Spawn Points`)))
  (`KismetArrayLibrary.Array_Shuffle` _output_get)
  (for _index (range (+ (`KismetMathLibrary.RandomIntegerInRange` 0 2) 1))
    (switch `int` (`KismetMathLibrary.RandomIntegerInRange` 0 2)
      (:`0`
        (bind _returnvalue (`KismetMathLibrary.MakeRelativeTransform` (`|GetArrayItem` (`local.Random Spawn Points`) _index) (`self.GetTransform`)))
        (`AddComponent|NODE_AddChildActorComponent-1` :`RelativeTransform` _returnvalue))
      (:`1`
        (`AddComponent|NODE_AddChildActorComponent-3` :`RelativeTransform` _returnvalue))
      (:`2`
        (`AddComponent|NODE_AddChildActorComponent-4` :`RelativeTransform` _returnvalue)))))

(fn `UserConstructionScript`
  (`self.Setup Spawn Points`)
  (`self.Spawn Obstacles`))